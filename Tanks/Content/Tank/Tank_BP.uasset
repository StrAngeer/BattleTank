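; Tank pawn Blueprint that wires player input to its aiming and movement components.
; On BeginPlay it hands the barrel and turret to TankAiming and both tracks to TankMovement.
; Mouse axes yaw the gimbal and pitch the spring arm for the camera, while Fire calls TankAiming.
; Forward/backward and left/right track axes are summed in pairs to feed IntendToMove and IntendToTurn.
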(event `self.ReceiveBeginPlay`
  (`TankAimingComponent.setBarrelAndTurret` (`self.TankAiming`) (`self.Barrel`) (`self.tankTurret`))
  (`tankMovementComponent.setTracks` (`self.tankMovement`) (`self.Left Track`) (`self.Right Track`)))

(event `InputAxis|Camera X from Mouse`
  (params (AxisValue :type "Float (single-precision)"))
  (`SceneComponent.K2_AddLocalRotation` (`self.Gimbal`) (`KismetMathLibrary.MakeRotator` 0.0 0.0 AxisValue) false false))

(event `InputAxis|Camera Y from mouse`
  (params (AxisValue :type "Float (single-precision)"))
  (`SceneComponent.K2_AddLocalRotation` (`self.SpringArm`) (`KismetMathLibrary.MakeRotator` 0.0 AxisValue) false false))

(event `InputAction|Fire`
  (params (Key :type "Key Structure"))
  (:`Pressed`
    (`TankAimingComponent.fire` (`self.TankAiming`))))

(event `InputAxis|Left Track Input`
  (params (AxisValue :type "Float (single-precision)"))
  (`tankMovementComponent.intendToTurn` (`self.tankMovement`) (+ (stale `InputAxis|Right Track Input` AxisValue) AxisValue) :!label _label))

(event `InputAxis|Right Track Input`
  (params (AxisValue :type "Float (single-precision)"))
  (goto _label))

(event `InputAxis|Forward input`
  (params (AxisValue :type "Float (single-precision)"))
  (`tankMovementComponent.intendToMove` (`self.tankMovement`) (+ (stale `InputAxis|Backward input` AxisValue) AxisValue) :!label _label_2))

(event `InputAxis|Backward input`
  (params (AxisValue :type "Float (single-precision)"))
  (goto _label_2))

(fn `UserConstructionScript`)